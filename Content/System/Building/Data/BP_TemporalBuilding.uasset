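; Base building Blueprint for buildings that perform an action repeatedly on a timer.
; Upgrading through UpLevel calls StartTimer, which clears any valid timer and sets a looping one at the level's delay to call Do.
; Pause and start events bound on BeginPlay pause or unpause that timer by handle.
; Do is empty and BufferIsEnough returns false, both apparently placeholders for child buildings.
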(event `self.ReceiveBeginPlay`
  (add `self.OnTimerPause` (delegate `OnTimerResetEvent`))
  (add `self.OnTimerStart` (delegate `OnTimerStartEvent`)))

(event `OnTimerResetEvent`
  (`self.PauseTimer`))

(event `OnTimerStartEvent`
  (`self.UnpauseTimer`))

(event `StartTimer`
  (bind _timerhandle (`self.TimerHandle`))
  (if (`KismetSystemLibrary.K2_IsValidTimerHandle` _timerhandle)
    (`KismetSystemLibrary.K2_ClearAndInvalidateTimerHandle` _timerhandle))
  (`KismetSystemLibrary.K2_SetTimerDelegate` (delegate `DoByBehavior`) (`/Game/System/Building/Data/PDA_BuildingLevel.Delay` (`self.Level`)) true))

(event `DoByBehavior`
  (`self.Do`))

(fn `BufferIsEnough`
  (params (Buffer :type "Map of /Game/System/Resource/Data/PDA_Resource Object Reference to Integer"))
  (returns (Success :type Boolean))
  (return false))

(fn `Do`)

(fn `PauseTimer`
  (`KismetSystemLibrary.K2_PauseTimerHandle` (`self.TimerHandle`)))

(fn `UnpauseTimer`
  (`KismetSystemLibrary.K2_UnPauseTimerHandle` (`self.TimerHandle`)))

(fn `UpLevel`
  (`parent.UpLevel`)
  (`self.StartTimer`))

(fn `UserConstructionScript`
  (`parent.UserConstructionScript`))