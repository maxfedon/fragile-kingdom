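; Recycling building that converts the current level's input resources into its output resources, extending a parent building's Do step.
; Each Do call checks that both resource sets fit their buffers, removes inputs from InputBuffer, adds outputs to OutputBuffer and writes a debug log.
; When the check fails, it calls OnTimerPause.
; BufferIsEmpty and BufferIsFull are stubs that always return false, so only the fit checks gate conversion.
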(fn `BufferIsEmpty`
  (params (Buffer :type "Map of /Game/System/Resource/Data/PDA_Resource Object Reference to Integer"))
  (returns (Success :type Boolean))
  (return false))

(fn `BufferIsFull`
  (params (Buffer :type "Map of /Game/System/Resource/Data/PDA_Resource Object Reference to Integer"))
  (returns (Success :type Boolean))
  (return false))

(fn `Do`
  (bind _level (`self.Level`))
  (`parent.Do`)
  (if (and (and (not (`self.BufferIsEmpty` (`self.InputBuffer`))) (not (`self.BufferIsFull` (`self.OutputBuffer`)))) (and (`self.FitsInBuffer` (`/Game/System/Building/Data/PDA_BuildingLevel.InputResources` _level) (`self.InputBuffer`)) (`self.FitsInBuffer` (`/Game/System/Building/Data/PDA_BuildingLevel.OutputResources` _level) (`self.OutputBuffer`))))
    (`self.RemoveFromBuffer` (`/Game/System/Building/Data/PDA_BuildingLevel.InputResources` (`self.Level`)) (`self.InputBuffer`))
    (`self.AddToBuffer` (`/Game/System/Building/Data/PDA_BuildingLevel.OutputResources` (`self.Level`)) (`self.OutputBuffer`))
    (`self.DEBUG_Log`)
    (return)
    (else
      (`self.OnTimerPause`))))

(fn `UserConstructionScript`
  (`parent.UserConstructionScript`))