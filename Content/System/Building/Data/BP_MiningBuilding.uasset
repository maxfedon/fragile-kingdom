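; BP_MiningBuilding is a child building Blueprint for mining that produces resources into its output buffer.
; Its Do step runs the parent logic, then adds the current Level's InputResources to OutputBuffer and logs on success.
; A full buffer or failed add calls OnTimerPause, although the BufferIsFull defined here always returns false, so only a failed add triggers it.
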(fn `BufferIsFull`
  (params (Buffer :type "Map of /Game/System/Resource/Data/PDA_Resource Object Reference to Integer"))
  (returns (Success :type Boolean))
  (return false))

(fn `Do`
  (`parent.Do`)
  (if (not (`self.BufferIsFull` (`self.OutputBuffer`)))
    (bind _success (`self.AddToBuffer` (`/Game/System/Building/Data/PDA_BuildingLevel.InputResources` (`self.Level`)) (`self.OutputBuffer`)))
    (if _success
      (`self.DEBUG_Log`)
      (return)
      (else
        (`self.OnTimerPause`)))
    (else
      (`self.OnTimerPause`))))

(fn `UserConstructionScript`
  (`parent.UserConstructionScript`))