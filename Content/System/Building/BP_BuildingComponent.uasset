(event Input|EnhancedActionEvents|EnhancedInputActionIA_BuildingRotate
  (params (ActionValue :type Float%20%28double-precision%29) (ElapsedSeconds :type Float%20%28double-precision%29) (TriggeredSeconds :type Float%20%28double-precision%29) (InputAction :type Input%20Action%20Object%20Reference :default "/Game/Player/Input/Action/Building/IA_BuildingRotate.IA_BuildingRotate"))
  (bind _preview (Variables|Default|GetPreview))
  ;[0.15 0.15 0.15 0.5] Rotate
  (Utilities|IsValid _preview
    (:Is%20Valid
      (Default|Rotate _preview ActionValue))))

(event Input|EnhancedActionEvents|EnhancedInputActionIA_BuildingPlace
  (params (ActionValue :type Boolean) (ElapsedSeconds :type Float%20%28double-precision%29) (TriggeredSeconds :type Float%20%28double-precision%29) (InputAction :type Input%20Action%20Object%20Reference :default "/Game/Player/Input/Action/Building/IA_BuildingPlace.IA_BuildingPlace"))
  ;[0.15 0.15 0.15 0.5] Place
  (:Started
    (if (CallFunction|CanBuild)
      (CallFunction|PlaceBuilding))))

(event Input|EnhancedActionEvents|EnhancedInputActionIA_BuildingCancel
  (params (ActionValue :type Boolean) (ElapsedSeconds :type Float%20%28double-precision%29) (TriggeredSeconds :type Float%20%28double-precision%29) (InputAction :type Input%20Action%20Object%20Reference :default "/Game/Player/Input/Action/Building/IA_BuildingCancel.IA_BuildingCancel"))
  ;[0.15 0.15 0.15 0.5] Cancel
  (:Started
    (CallFunction|RemovePreview)))

(event EventTick
  (params (DeltaSeconds :type Float%20%28single-precision%29))
  ;[0.15 0.15 0.15 0.5] Tick: Handle Preview
  (Utilities|IsValid (Variables|Default|GetPreview)
    (:Is%20Valid
      (CallFunction|HandlePreview))))

(event Input|KeyboardEvents|DebugKeyZ
  (params (Key :type Key%20Structure :default "None") (ActionValue :type Input%20Action%20Value%20Structure))
  (:Pressed
    (CallFunction|CreatePreview "/Game/System/Building/Data/Warehouse/DA_Warehouse.DA_Warehouse" "0, 0, 0")))

(event Input|KeyboardEvents|DebugKeyX
  (params (Key :type Key%20Structure :default "None") (ActionValue :type Input%20Action%20Value%20Structure))
  (:Pressed
    (CallFunction|CreatePreview "/Game/System/Building/Data/Farm/DA_Farm.DA_Farm" "0, 0, 0")))

(fn Init
  (params (PlayerController :type BP%20Player%20Controller%20Object%20Reference))
  (bind _output_get (Variables|Components|SetPlayerController PlayerController))
  ;[0.15 0.15 0.15 0.5] BuildingMenu
  (bind _returnvalue (UserInterface|CreateWidget "/Game/UI/Building/W_BuildingMenu.W_BuildingMenu_C"))
  (Default|AddWidget (Variables|/Game/Player/BP_PlayerController.BP_PlayerController_C|GetHUD _output_get) _returnvalue false)
  (bind _output_get_2 (Variables|Widget|SetBuildingWidget _returnvalue))
  (Default|Init _output_get_2)
  ;[0.15 0.15 0.15 0.5] Warning
  (bind _returnvalue_2 (UserInterface|CreateWidget "/Game/UI/Building/W_BuildingWarning.W_BuildingWarning_C" 0 "Too far away!"))
  (bind _output_get_3 (Variables|Widget|SetWarningWidget _returnvalue_2))
  (Default|AddWidget (Variables|/Game/Player/BP_PlayerController.BP_PlayerController_C|GetHUD _output_get) _output_get_3 true))

(fn Build
  (params (BuildingAsset :type PDA%20Building%20Object%20Reference))
  (CallFunction|CreatePreview BuildingAsset (.Location (Default|GetLookPoint (Variables|Components|GetPlayerController)))))

(fn CreatePreview
  (params (BuildingAsset :type PDA%20Building%20Object%20Reference) (Position :type Vector))
  (CallFunction|RemovePreview)
  (bind _returnvalue (Game|SpawnActorfromClass "/Game/System/Building/BP_BuildingPreview.BP_BuildingPreview_C" (Math|Transform|MakeTransform Position "0, 0, 0" "1.000000,1.000000,1.000000") "Undefined" "MultiplyWithRoot" 0 BuildingAsset 0))
  (Variables|Default|SetPreview _returnvalue))

(fn HandlePreview
  (bind _playercontroller (Variables|Components|GetPlayerController))
  (bind _preview (Variables|Default|GetPreview))
  (bind _preview_2 (Variables|Default|GetPreview))
  (bind (_hit _location) (Default|GetLookPoint _playercontroller))
  (if _hit
    (Utilities|DistanceVisibility _preview false "Hidden")
    (Transformation|SetActorLocation _preview (Math|Vector|MakeVector (.x _location) (.y _location) (.z (Transformation|GetActorLocation _preview))) false false)
    (if (CallFunction|CanBuild)
      (Default|ChangeState _preview_2 "NewEnumerator0")
      (else
        (Default|ChangeState _preview_2 "NewEnumerator1")))
    (else
      (Utilities|DistanceVisibility _preview true "Visible"))))

(fn RemovePreview
  (Utilities|IsValid (Variables|Default|GetPreview)
    (:Is%20Valid
      (Actor|DestroyActor (Variables|Default|GetPreview))
      (Variables|Default|SetPreview 0))))

(fn PlaceBuilding
  (bind _preview (Variables|Default|GetPreview))
  (Utilities|IsValid _preview
    (:Is%20Valid
      (Game|SpawnActorfromClass "/Game/System/Building/BP_Building.BP_Building_C" (Transformation|GetActorTransform _preview) "Undefined" "MultiplyWithRoot" 0 (Variables|/Game/System/Building/BP_BuildingPreview.BP_BuildingPreview_C|GetBuildingAsset _preview) 0)
      (CallFunction|RemovePreview))))

(fn CanBuild
  (bind _preview (Variables|Default|GetPreview))
  (Utilities|IsValid _preview
    (:Is%20Valid
      (return (== (Utilities|Array|Length (Class|PrimitiveComponent|GetOverlappingComponents (Variables|/Game/System/Building/BP_BuildingPreview.BP_BuildingPreview_C|GetPreviewMesh _preview))) 0)))))

(fn GetLocationUnderCursor)