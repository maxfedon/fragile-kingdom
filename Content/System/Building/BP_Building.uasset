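; Building actor configured from a BuildingAsset, with levels and input and output resource buffers.
; The construction script applies the first level's mesh and the asset's radius to a sphere, then calls UpLevel to advance the level index and data.
; Map helpers add or subtract resource counts, removing entries at zero, and a debug function prints both buffers.
; AddResources and the empty, full and fit checks are unimplemented stubs.
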(fn `AddResources`
  (params (Resources :type "Map of /Game/System/Resource/Data/PDA_Resource Object Reference to Integer"))
  (returns (Remainder :type "Map of /Game/System/Resource/Data/PDA_Resource Object Reference to Integer") (Success :type Boolean)))

(fn `AddToBuffer`
  (params (Resources :type "Map of /Game/System/Resource/Data/PDA_Resource Object Reference to Integer") (Buffer :type "Map of /Game/System/Resource/Data/PDA_Resource Object Reference to Integer (by ref)"))
  (locals (CurrentResource :type "/Game/System/Resource/Data/PDA_Resource Object Reference") (CurrentCount :type Integer))
  (bind (_value _returnvalue) (`BlueprintMapLibrary.Map_Find` (`local.Buffer`) (`local.CurrentResource`)))
  (bind (_keypin _valuepin) (`|MapForEach` Resources)
    (:`then`
      (set `local.CurrentResource` _keypin)
      (set `local.CurrentCount` _valuepin)
      (if _returnvalue
        (`BlueprintMapLibrary.Map_Add` (`local.Buffer`) (`local.CurrentResource`) (+ _value (`local.CurrentCount`)))
        (else
          (`BlueprintMapLibrary.Map_Add` (`local.Buffer`) (`local.CurrentResource`) (`local.CurrentCount`)))))))

(fn `BufferIsEmpty`
  (params (Buffer :type "Map of /Game/System/Resource/Data/PDA_Resource Object Reference to Integer"))
  (returns (Success :type Boolean))
  (return false))

(fn `BufferIsFull`
  (params (Buffer :type "Map of /Game/System/Resource/Data/PDA_Resource Object Reference to Integer"))
  (returns (Success :type Boolean))
  (return false))

(fn `DEBUG_Log`
  (`KismetSystemLibrary.PrintString` "---------------------")
  (bind (_keypin _valuepin) (`|MapForEach` (`self.InputBuffer`))
    (:`then`
      (`KismetSystemLibrary.PrintString` (`KismetStringLibrary.Concat_StrStr` "R_I | " (`KismetSystemLibrary.GetDisplayName` _keypin) ": " (`KismetStringLibrary.Conv_IntToString` _valuepin))))
    (:`CompletedPin`
      (`KismetSystemLibrary.PrintString` "---")
      (bind (_keypin_2 _valuepin_2) (`|MapForEach` (`self.OutputBuffer`))
        (:`then`
          (`KismetSystemLibrary.PrintString` (`KismetStringLibrary.Concat_StrStr` "R_O | " (`KismetSystemLibrary.GetDisplayName` _keypin_2) ": " (`KismetStringLibrary.Conv_IntToString` _valuepin_2))))
        (:`CompletedPin`
          (`KismetSystemLibrary.PrintString` "---------------------"))))))

(fn `FitsInBuffer`
  (params (Resources :type "Map of /Game/System/Resource/Data/PDA_Resource Object Reference to Integer") (Buffer :type "Map of /Game/System/Resource/Data/PDA_Resource Object Reference to Integer"))
  (returns (Success :type Boolean))
  (return false))

(fn `RemoveFromBuffer`
  (params (Resources :type "Map of /Game/System/Resource/Data/PDA_Resource Object Reference to Integer") (Buffer :type "Map of /Game/System/Resource/Data/PDA_Resource Object Reference to Integer"))
  (locals (CurrentResource :type "/Game/System/Resource/Data/PDA_Resource Object Reference") (CurrentCount :type Integer) (ModifyBuffer :type "Map of /Game/System/Resource/Data/PDA_Resource Object Reference to Integer"))
  (bind (_keypin _valuepin) (`|MapForEach` Resources)
    (:`then`
      (set `local.CurrentResource` _keypin)
      (set `local.CurrentCount` _valuepin)
      (`BlueprintMapLibrary.Map_Add` (`local.Buffer`) (`local.CurrentResource`) (- (`BlueprintMapLibrary.Map_Find` (`local.Buffer`) (`local.CurrentResource`)) (`local.CurrentCount`)))
      (if (== (`BlueprintMapLibrary.Map_Find` (`local.Buffer`) (`local.CurrentResource`)) 0)
        (`BlueprintMapLibrary.Map_Remove` (`local.Buffer`) (`local.CurrentResource`))))))

(fn `UpLevel`
  (bind _result (`/Engine/EditorBlueprintResources/StandardMacros.IncrementInt` (`self.LevelIndex`))
    (:`  `
      (set `self.Level` (`|GetArrayItem` (`/Game/System/Building/Data/PDA_Building.Levels` (`self.BuildingAsset`)) _result)))))

(fn `UserConstructionScript`
  (bind _buildingasset (`self.BuildingAsset`)
    (:`then`
      ; StaticMesh
      (`StaticMeshComponent.SetStaticMesh` (`self.StaticMesh`) (`/Game/System/Building/Data/PDA_BuildingLevel.Mesh` (`|GetArrayItem` (`/Game/System/Building/Data/PDA_Building.Levels` _buildingasset))))
      ; SphereCollision radius
      (`SphereComponent.SetSphereRadius` (`self.Radius`) (`/Game/System/Building/Data/PDA_Building.Radius` (`self.BuildingAsset`)) true)
      (`self.UpLevel`))
    (:`else`)))