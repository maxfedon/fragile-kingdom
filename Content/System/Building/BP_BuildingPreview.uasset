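; Placement preview actor for buildings, showing the first-level mesh from its building asset.
; Construction sets that mesh, applies the positive material and gives it a random starting yaw.
; ChangeState swaps every material slot between positive and negative materials, only when the state changes.
; Rotate turns the actor around yaw in 11.25-degree steps, though the random start uses fractional steps, so yaw is not grid-aligned.
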(fn `ChangeState`
  (params (NewState :type "/Game/System/Building/E_BuildingPreviewState Enum" :default "NewEnumerator0"))
  (locals (NewLocalVar :type Byte :default 0))
  (if (`|EnumInequality` NewState (`self.BuildingPreviewState`))
    (bind _output_get (set `self.BuildingPreviewState` (`local.NewState`)))
    (`self.SetPreviewMaterial` _output_get)))

(fn `Rotate`
  (params (Step :type "Float (double-precision)"))
  (`self.K2_AddActorWorldRotation` (`KismetMathLibrary.MakeRotator` 0.0 0.0 (* Step 11.25))))

(fn `SetPreviewMaterial`
  (params (NewState :type "/Game/System/Building/E_BuildingPreviewState Enum" :default "NewEnumerator0"))
  (locals (Material :type "Material Object Reference") (Meshes :type "Array of MeshComponent Object Reference"))
  (bind _previewmesh (`self.PreviewMesh`))
  (switch `/Game/System/Building/E_BuildingPreviewState` NewState
    (:`NewEnumerator0`
      (set `local.Material` (`self.PositiveMaterial`)))
    (:`NewEnumerator1`
      (set `local.Material` (`self.NegativeMaterial`))))
  (for _index (range (+ (`PrimitiveComponent.GetNumMaterials` _previewmesh) 1))
    (`PrimitiveComponent.SetMaterial` _previewmesh _index (`local.Material`))))

(fn `UserConstructionScript`
  (`StaticMeshComponent.SetStaticMesh` (`self.PreviewMesh`) (`/Game/System/Building/Data/PDA_BuildingLevel.Mesh` (`|GetArrayItem` (`/Game/System/Building/Data/PDA_Building.Levels` (`self.BuildingAsset`)))))
  (`self.SetPreviewMaterial` "NewEnumerator0")
  ; Default rotate
  (`self.Rotate` (`KismetMathLibrary.RandomFloatInRange` -32.0 32.0)))